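; A six-degrees-of-freedom pawn that the player flies through axis input, moving and rotating its BodyMesh.
; MoveForward and MoveRight set physics linear velocity along the mesh's own forward and right vectors at a fixed speed scale.
; Forward input adds to the current velocity, while right input replaces it outright.
; LookUp, Turn and Roll apply raw axis values as local pitch, yaw and roll, without delta-time scaling.
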(event `InputAxis|MoveForward`
  (params (AxisValue :type "Float (single-precision)"))
  (`PrimitiveComponent.SetPhysicsLinearVelocity` (`self.BodyMesh`) (* (`KismetMathLibrary.GetForwardVector` (`SceneComponent.K2_GetComponentRotation` (`self.BodyMesh`))) (* AxisValue 300.0)) true "None"))

(event `InputAxis|MoveRight`
  (params (AxisValue :type "Float (single-precision)"))
  (`PrimitiveComponent.SetPhysicsLinearVelocity` (`self.BodyMesh`) (* (`KismetMathLibrary.GetRightVector` (`SceneComponent.K2_GetComponentRotation` (`self.BodyMesh`))) (* AxisValue 300.0)) false "None"))

(event `InputAxis|LookUp`
  (params (AxisValue :type "Float (single-precision)"))
  (`SceneComponent.K2_AddLocalRotation` (`self.BodyMesh`) (`KismetMathLibrary.MakeRotator` 0.0 AxisValue) false false))

(event `InputAxis|Turn`
  (params (AxisValue :type "Float (single-precision)"))
  (`SceneComponent.K2_AddLocalRotation` (`self.BodyMesh`) (`KismetMathLibrary.MakeRotator` 0.0 0.0 AxisValue) false false))

(event `InputAxis|Roll`
  (params (AxisValue :type "Float (single-precision)"))
  (`SceneComponent.K2_AddLocalRotation` (`self.BodyMesh`) (`KismetMathLibrary.MakeRotator` AxisValue) false false))

(fn `UserConstructionScript`)